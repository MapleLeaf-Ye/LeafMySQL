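; DataContentObj_BP is a data object in the DB editor that wraps one content entry and its selection and text state.
; InitObj stores new content, clears the selection and text maps, and unbinds all listeners from its selection and data-change event dispatchers.
; UpdateObj replaces the content and copies each value into the text map keyed by index, without clearing the map first.
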(fn InitObj
  (params (NewContent :type ES%20Row%20Content%20Structure))
  (Variables|Default|SetContent NewContent)
  (Utilities|Map|Clear (Variables|Default|GetIndexSelectState))
  (Utilities|Map|Clear (Variables|Default|GetCurrentTextContent))
  (Utilities|FlowControl|Sequence
    (:then_1
      (EventDispatchers|UnbindallEventsfromOnSelected)
      (EventDispatchers|UnbindallEventsfromOnDataChange)
      (EventDispatchers|UnbindallEventsfromOnUpdateSelectedState)
      (EventDispatchers|UnbindallEventsfromOnSelectGridChange)
      (EventDispatchers|UnbindallEventsfromOnContentUpdate))))

(fn UpdateObj
  (params (NewContent :type ES%20Row%20Content%20Structure))
  (bind _output_get (Variables|Default|SetContent NewContent))
  (for (_array_element _array_index) (.Values (Utilities|Struct|BreakES_RowContent _output_get))
    (Utilities|Map|Add (Variables|Default|GetCurrentTextContent) _array_index _array_element)))