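; Manager behind a MySQL database editor, wrapping a registered SQL Accessor for table browsing, editing and CSV import/export.
; It caches system info, database names, the selected table's structure and row-limited data, then fires dispatchers as these change.
; Row edits become inserts, updates or deletes by SaveState, using primary-key WHERE strings for the latter two.
; Accessor results mostly pass through CheckError, which broadcasts errors; CSV export runs asynchronously and prints progress.
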(event Custom|ExportData_Async
  (params (InFileExportPath :type String) (InTableName :type String) (InLimitRowNum :type Integer64))
  (bind (_asynctaskproxy _currentstate _currenthandlecount _targethandlecount _outerror) (|ExportDatatoCSVAsync (Variables|Default|GetAccessor) InFileExportPath InTableName InLimitRowNum)
    (:OnUpdateStateAndCount
      (Development|PrintString 0 (Utilities|String|Append (Utilities|String|EnumtoString _currentstate) "-" (Utilities|String|ToString(Integer) _currenthandlecount) "-" (Utilities|String|ToString(Integer) _targethandlecount) "-" _outerror)))))

(fn RegisterSQLAccessor
  (params (Accessor :type Leaf%20My%20SQL%20Accessor%20Base%20Object%20Reference) (Error :type String))
  (bind _output_get (Variables|Default|SetAccessor Accessor))
  (bind _sueccssed (CallFunction|CheckError Error))
  (if _sueccssed
    (Utilities|IsValid _output_get
      (:Is%20Valid
        (CallFunction|InitialManagerInfo)))))

(fn CheckError
  (params (Error :type String))
  (bind _returnvalue (Utilities|Array|IsEmpty Error))
  (bind _returnvalue_2 (Utilities|Enum|Equal(Enum) Error "successed"))
  (bind _returnvalue_3 (or _returnvalue _returnvalue_2))
  (Utilities|FlowControl|Sequence
    (:then_0
      (if (not _returnvalue_3)
        (Default|CallOnErrorThrow Error)
        (else
          (Default|CallOnErrorThrow))))
    (:then_1
      (return _returnvalue_3))))

(fn InitialManagerInfo
  (Utilities|FlowControl|Sequence
    (:then_0
      (Variables|Default|SetSQLSystemDetail (.OutSystemDetail (Class|LeafMySQLAccessorBase|ShowSystemDetail (Variables|Default|GetAccessor)))))
    (:then_1
      (Variables|Default|SetDataBases (.OutDataBaseNames (Class|LeafMySQLAccessorBase|ShowAllDataBase (Variables|Default|GetAccessor)))))
    (:then_2
      (Default|CallOnManagerInfoInitialOver))))

(fn ChangeTable
  (params (InTableName :type String))
  (bind _accessor (Variables|Default|GetAccessor))
  (bind (_outdatatablestructure _returnvalue) (Class|LeafMySQLAccessorBase|ShowDataTableStructure _accessor InTableName))
  (Variables|Default|SetPreTableName (Variables|Default|GetCacheTableName))
  (Variables|Default|SetCacheTableName InTableName)
  (Utilities|FlowControl|Sequence
    (:then_0
      (bind _sueccssed (CallFunction|CheckError _returnvalue))
      (if _sueccssed
        (Variables|Default|SetData%20Table%20Structure _outdatatablestructure)))
    (:then_1
      (bind (_outselecteddatas _returnvalue_2) (Class|LeafMySQLAccessorBase|FindDatafromTable _accessor InTableName (Utilities|Array|MakeArray "*") "(WhereString=\"None\")" "None" true (Variables|Default|GetLimitRowNum)))
      (bind _sueccssed_2 (CallFunction|CheckError _returnvalue_2))
      (if _sueccssed_2
        (Variables|Default|SetTableDatas _outselecteddatas)))
    (:then_2
      (Default|CallOnNewTableSelected (Variables|Default|GetCacheTableName)))))

(fn RefreshTable
  (bind _accessor (Variables|Default|GetAccessor))
  (bind _cachetablename (Variables|Default|GetCacheTableName))
  (bind (_outdatatablestructure _returnvalue) (Class|LeafMySQLAccessorBase|ShowDataTableStructure _accessor _cachetablename))
  (Utilities|FlowControl|Sequence
    (:then_0
      (bind _sueccssed (CallFunction|CheckError _returnvalue))
      (if _sueccssed
        (Variables|Default|SetData%20Table%20Structure _outdatatablestructure)))
    (:then_1
      (bind (_outselecteddatas _returnvalue_2) (Class|LeafMySQLAccessorBase|FindDatafromTable _accessor _cachetablename (Utilities|Array|MakeArray "*") "(WhereString=\"None\")" "None" true (Variables|Default|GetLimitRowNum)))
      (bind _sueccssed_2 (CallFunction|CheckError _returnvalue_2))
      (if _sueccssed_2
        (Variables|Default|SetTableDatas _outselecteddatas)))
    (:then_2
      (Default|CallOnRefresh))))

(fn AddNewRow
  (Default|CallOnAddNewRow))

(fn SyncDataBase
  (params (RowContent :type ES%20Row%20Content%20Structure))
  (bind _data_table_structure (Variables|Default|GetData%20Table%20Structure))
  (bind _data_table_structure_2 (Variables|Default|GetData%20Table%20Structure))
  (bind _data_table_structure_3 (Variables|Default|GetData%20Table%20Structure))
  (switch Utilities|FlowControl|Switch|SwitchonEE_SaveState (.SaveState (Utilities|Struct|BreakES_RowContent RowContent))
    (:NewEnumerator1
      (bind _keys (Utilities|Map|Keys _data_table_structure_3))
      (for (_array_element _array_index) _keys
        (if (not (.AutoIncrement (Utilities|Struct|BreakLeafColumnStructureDisplay (.Value (Utilities|Map|Find _data_table_structure_3 _array_element)))))
          (Utilities|Map|Add (LocalVariables|GetAddInfo) _array_element (Utilities|Array|Get(acopy) (.Values (Utilities|Struct|BreakES_RowContent RowContent)) _array_index))))
      (bind _returnvalue (Class|LeafMySQLAccessorBase|InsertDatatoTable (Variables|Default|GetAccessor) (Variables|Default|GetCacheTableName) (LocalVariables|GetAddInfo)))
      (CallFunction|CheckError _returnvalue))
    (:NewEnumerator2
      (bind _keys_2 (Utilities|Map|Keys _data_table_structure_2))
      (for (_array_element_2 _array_index_2) _keys_2
        (if (.IsPrimaryKey (Utilities|Struct|BreakLeafColumnStructureDisplay (.Value (Utilities|Map|Find _data_table_structure_2 _array_element_2))))
          (LocalVariables|SetCondition (Utilities|String|Append (.ColumnName (Utilities|Struct|BreakLeafColumnStructureDisplay (.Value (Utilities|Map|Find _data_table_structure_2 _array_element_2)))) "=" "'" (Utilities|Array|Get(acopy) (.Values (Utilities|Struct|BreakES_RowContent RowContent)) _array_index_2) "'"))))
      (bind _returnvalue_2 (Class|LeafMySQLAccessorBase|DeleteDatafromTable (Variables|Default|GetAccessor) (Variables|Default|GetCacheTableName) (Utilities|Struct|MakeLeafSQLWhereString (LocalVariables|GetCondition))))
      (CallFunction|CheckError _returnvalue_2))
    (:NewEnumerator3
      (bind _keys_3 (Utilities|Map|Keys _data_table_structure))
      (for (_array_element_3 _array_index_3) _keys_3
        (if (.IsPrimaryKey (Utilities|Struct|BreakLeafColumnStructureDisplay (.Value (Utilities|Map|Find _data_table_structure _array_element_3))))
          (LocalVariables|SetCondition (Utilities|String|Append (.ColumnName (Utilities|Struct|BreakLeafColumnStructureDisplay (.Value (Utilities|Map|Find _data_table_structure _array_element_3)))) "=" "'" (Utilities|Array|Get(acopy) (.Values (Utilities|Struct|BreakES_RowContent RowContent)) _array_index_3) "'"))
          (else
            (Utilities|Map|Add (LocalVariables|GetAddInfo) _array_element_3 (Utilities|Array|Get(acopy) (.Values (Utilities|Struct|BreakES_RowContent RowContent)) _array_index_3)))))
      (bind _returnvalue_3 (Class|LeafMySQLAccessorBase|UpdateDatafromTable (Variables|Default|GetAccessor) (Variables|Default|GetCacheTableName) (LocalVariables|GetAddInfo) (Utilities|Struct|MakeLeafSQLWhereString (LocalVariables|GetCondition))))
      (CallFunction|CheckError _returnvalue_3))))

(fn FindRow
  (params (FilterCommand :type String))
  (if (Utilities|Array|IsEmpty FilterCommand)
    (CallFunction|RefreshTable)
    (else
      (bind (_outselecteddatas _returnvalue) (Class|LeafMySQLAccessorBase|FindDatafromTable (Variables|Default|GetAccessor) (Variables|Default|GetCacheTableName) (Utilities|Array|MakeArray "*") (Utilities|Struct|MakeLeafSQLWhereString FilterCommand) "None" true (Variables|Default|GetLimitRowNum)))
      (bind _sueccssed (CallFunction|CheckError _returnvalue))
      (if _sueccssed
        (Variables|Default|SetTableDatas _outselecteddatas)
        (Default|CallOnRefresh)))))

(fn DeConnect
  (bind _accessor (Variables|Default|GetAccessor)
    (:then
      (Class|LeafMySQLAccessorBase|DeConnectMySQL _accessor)
      (Utilities|Map|Clear (Variables|Default|GetSQLSystemDetail))
      (Utilities|Map|Clear (Variables|Default|GetData%20Table%20Structure))
      (Utilities|Array|Clear (Variables|Default|GetDataBases))
      (Utilities|Array|Clear (Variables|Default|GetTableDatas))
      (Default|CallOnDeConnect))
    (:else)))

(fn OriderRow
  (params (ColumnName :type String) (bInIsASC :type Boolean))
  (if (Utilities|Array|IsEmpty ColumnName)
    (CallFunction|CheckError "Column is empty!")
    (else
      (bind (_outselecteddatas _returnvalue) (Class|LeafMySQLAccessorBase|FindDatafromTable (Variables|Default|GetAccessor) (Variables|Default|GetCacheTableName) (Utilities|Array|MakeArray) "(WhereString=\"None\")" ColumnName bInIsASC (Variables|Default|GetLimitRowNum)))
      (bind _sueccssed (CallFunction|CheckError _returnvalue))
      (if _sueccssed
        (Variables|Default|SetTableDatas _outselecteddatas)
        (Default|CallOnRefresh)))))

(fn UpdateRowLimit
  (params (NewLimitRowNum :type Integer64))
  (Variables|Default|SetLimitRowNum NewLimitRowNum)
  (CallFunction|RefreshTable))

(fn ExportData
  (params (FileExportPath :type String))
  (if (Utilities|Array|IsEmpty (Variables|Default|GetCacheTableName))
    (CallFunction|CheckError "Path dont contain .csv file at end")
    (elif (Utilities|String|EndsWith FileExportPath ".csv")
      (Variables|Default|SetFileExportPath FileExportPath)
      (CallFunction|ExportDataAsync (Variables|Default|GetFileExportPath) (Variables|Default|GetCacheTableName) (Variables|Default|GetLimitRowNum))
      (else
        (CallFunction|CheckError "Path dont contain .csv file at end")))))

(fn ImportData
  (params (FileImportPath :type String) (OverrideSourceData :type Boolean))
  (if (Utilities|Array|IsEmpty (Variables|Default|GetCacheTableName))
    (CallFunction|CheckError "Dont select any table")
    (elif (Utilities|String|EndsWith FileImportPath ".csv")
      (Variables|Default|SetFileExportPath FileImportPath)
      (bind _returnvalue (Class|LeafMySQLAccessorBase|ImportDatatoDataTablefromCSV (Variables|Default|GetAccessor) (Variables|Default|GetFileExportPath) (Variables|Default|GetCacheTableName) OverrideSourceData))
      (bind _sueccssed (CallFunction|CheckError _returnvalue))
      (if _sueccssed
        _
        (else
          _))
      (CallFunction|RefreshTable)
      (else
        (CallFunction|CheckError "Path dont contain .csv file at end")))))

(fn DeleteDataTable
  (params (JustData :type Boolean))
  (bind _accessor (Variables|Default|GetAccessor))
  (bind (_outdatatablenames _returnvalue) (Class|LeafMySQLAccessorBase|ShowCurrentDataBaseAllTable _accessor))
  (bind _returnvalue_2 (Class|LeafMySQLAccessorBase|DeleteDataTable (Variables|Default|GetAccessor) (Variables|Default|GetCacheTableName) true JustData))
  (bind _sueccssed (CallFunction|CheckError _returnvalue_2))
  (if _sueccssed
    (if JustData
      (CallFunction|RefreshTable)
      (else
        (bind _sueccssed_2 (CallFunction|CheckError _returnvalue))
        (if (and _sueccssed_2 (> (Utilities|Array|Length _outdatatablenames) 0))
          (CallFunction|ChangeTable (Utilities|Array|Get(acopy) _outdatatablenames))
          (Default|CallOnDeleteTable)
          (CallFunction|RefreshTable)
          (else
            (CallFunction|DeConnect)))))))